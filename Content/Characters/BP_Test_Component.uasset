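; BP_Test_Component is a test actor component that drives a GAS jump on its owning Character.
; On BeginPlay it caches the owner's ability system, Character and movement component, and Jump input activates the GA_Test_AnimInstance_Jump ability.
; Tick prints the movement mode and detects landing by polling for a Falling-to-Walking change, then sends a Landed gameplay event, a stopgap for being unable to bind OnLanded.
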(event `self.ReceiveBeginPlay`
  (set `self.OwnerASC` (`AbilitySystemBlueprintLibrary.GetAbilitySystemComponent` (`self.GetOwner`)))
  (bind _ascharacter (cast `Character` (`self.GetOwner`)))
  (bind _output_get (set `self.OwnerCharacter` _ascharacter))
  (set `self.OwnerCMC` (`Character.CharacterMovement` _output_get)))

(event `InputAction|Jump`
  (params (Key :type "Key Structure"))
  (:`Pressed`
    (`AbilitySystemComponent.TryActivateAbilityByClass` (`self.OwnerASC`) "/GASCompanionTests/Tests/AnimInstance/Abilities/GA_Test_AnimInstance_Jump.GA_Test_AnimInstance_Jump_C" true)))

(event `self.ReceiveTick`
  (params (DeltaSeconds :type "Float (single-precision)"))
  ;[0.6844 0.4945 0.1799] Note: Not able to bind OnLanded event from there, has to be done in Owner Character unfortunately
  ;
  ; TODO: Consider project specific PawnComponent that exposes that.
  ;
  ; Right now, quick and dirty monitoring of CMC's MovementMode
  (`KismetSystemLibrary.PrintText` (`|FormatText` "Actor Component: {Character} - {Mode}" (`self.OwnerCharacter`) (`|GetEnumeratorNameAsString` (`CharacterMovementComponent.MovementMode` (`self.OwnerCMC`)))) true false (struct :`G` 0.66 :`B` 1.0 :`A` 1.0) 0.0)
  (`|ExecutionSequence`
    (:`then_0`
      (switch `EMovementMode` (`self.PrevMovementMode`)
        (:`MOVE_Falling`
          (if (`|EnumEquality` (`CharacterMovementComponent.MovementMode` (`self.OwnerCMC`)) "MOVE_Walking")
            (`AbilitySystemBlueprintLibrary.SendGameplayEventToActor` (`self.OwnerCharacter`) (struct :`TagName` "GASCompanionTests.Event.Landed"))))))
    (:`then_1`
      (set `self.PrevMovementMode` (`CharacterMovementComponent.MovementMode` (`self.OwnerCMC`))))))